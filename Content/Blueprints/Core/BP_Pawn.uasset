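; Player-controlled airplane pawn that flies forward constantly through FloatingPawnMovement, with pitch, roll, rocket fire and boost.
; Pitch and Roll axes apply frame-rate-scaled local rotation, and Fire spawns BP_Rocket at the pawn's transform.
; Boost press and release run separate timelines that shorten or restore the spring arm, changing max speed and deceleration only when each finishes.
; A BoostTime function sets speed and acceleration but is not called in this graph.
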(event EventTick
  (params (DeltaSeconds :type Float%20%28single-precision%29))
  ;[0.15 0.15 0.15 0.5] 비행기 이동
  (Pawn|Input|AddMovementInput (Transformation|GetActorForwardVector) (Variables|Default|GetBoostSpeed) false))

(event Input|ActionEvents|InputActionFire
  (params (Key :type Key%20Structure :default "None"))
  ;[0.15 0.15 0.15 0.5] 로켓 스폰.
  (:Pressed
    (Game|SpawnActorfromClass "/Game/Blueprints/Actor/BP_Rocket.BP_Rocket_C" (Transformation|GetActorTransform) "Undefined" "MultiplyWithRoot" 0 0)))

(event Input|ActionEvents|InputActionBoost
  (params (Key :type Key%20Structure :default "None"))
  (bind _floatingpawnmovement (Variables|Default|GetFloatingPawnMovement))
  (bind _floatingpawnmovement_2 (Variables|Default|GetFloatingPawnMovement))
  (bind _springarm (Variables|Default|GetSpringArm))
  ;[0.15 0.15 0.15 0.5] 부스터 기능
  (:Pressed
    (bind _alpha (Timeline|Timeline PlayFromStart)
      (:Update
        (Variables|/Script/Engine.SpringArmComponent|SetTargetArmLength _springarm (Math|Float|Lerp 1.5e+02 5e+01 _alpha)))
      (:Finished
        (Variables|/Script/Engine.FloatingPawnMovement|SetMaxSpeed _floatingpawnmovement 2.4e+03)
        (Variables|/Script/Engine.FloatingPawnMovement|SetDeceleration _floatingpawnmovement 2e+02))))
  (:Released
    (bind _alpha_2 (Timeline|Timeline_0 PlayFromStart)
      (:Update
        (Variables|/Script/Engine.SpringArmComponent|SetTargetArmLength _springarm (Math|Float|Lerp 5e+01 1.5e+02 _alpha_2)))
      (:Finished
        (Variables|/Script/Engine.FloatingPawnMovement|SetMaxSpeed _floatingpawnmovement_2 1.2e+03)
        (Variables|/Script/Engine.FloatingPawnMovement|SetDeceleration _floatingpawnmovement_2 6e+02)))))

(event Input|AxisEvents|InputAxisPitch
  (params (AxisValue :type Float%20%28single-precision%29))
  ;[0.15 0.15 0.15 0.5] 비행기 회전
  (Transformation|AddActorLocalRotation (Math|Rotator|MakeRotator 0.0 (* AxisValue (Utilities|Time|GetWorldDeltaSeconds) (Variables|Default|GetRotationSpeed)) 0.0) false false))

(event Input|AxisEvents|InputAxisRoll
  (params (AxisValue :type Float%20%28single-precision%29))
  ;[0.15 0.15 0.15 0.5] 비행기 회전
  (Transformation|AddActorLocalRotation (Math|Rotator|MakeRotator (* AxisValue (Utilities|Time|GetWorldDeltaSeconds) (Variables|Default|GetRotationSpeed)) 0.0 0.0) false false))

(fn ConstructionScript)

(fn BoostTime
  (bind _floatingpawnmovement (Variables|Default|GetFloatingPawnMovement))
  (Variables|/Script/Engine.FloatingPawnMovement|SetMaxSpeed _floatingpawnmovement 2.4e+03)
  (Variables|/Script/Engine.FloatingPawnMovement|SetAcceleration _floatingpawnmovement 2e+02))