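; BP_Pawn is a player-controlled airplane pawn that flies forward constantly and fires rockets.
; Tick feeds forward movement input to FloatingPawnMovement, while Pitch and Roll axes apply frame-rate-scaled local rotation.
; Fire spawns BP_Rocket at the actor's transform, and holding Boost raises max speed and lowers deceleration until release.
; A separate BoostTime function sets a higher max speed and changes acceleration, but nothing in this Blueprint calls it.
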(event EventTick
  (params (DeltaSeconds :type Float%20%28single-precision%29))
  ;[0.15 0.15 0.15 0.5] 비행기 이동
  (Pawn|Input|AddMovementInput (Transformation|GetActorForwardVector) 1.0 false))

(event Input|ActionEvents|InputActionFire
  (params (Key :type Key%20Structure :default "None"))
  ;[0.15 0.15 0.15 0.5] 로켓 스폰.
  (:Pressed
    (Game|SpawnActorfromClass "/Game/Actor/BP_Rocket.BP_Rocket_C" (Transformation|GetActorTransform) "Undefined" "MultiplyWithRoot" 0 0)))

(event Input|ActionEvents|InputActionBoost
  (params (Key :type Key%20Structure :default "None"))
  (bind _floatingpawnmovement (Variables|Default|GetFloatingPawnMovement))
  (bind _floatingpawnmovement_2 (Variables|Default|GetFloatingPawnMovement))
  ;[0.15 0.15 0.15 0.5] 부스터 기능
  (:Pressed
    (Variables|/Script/Engine.FloatingPawnMovement|SetMaxSpeed _floatingpawnmovement 1.2e+03)
    (Variables|/Script/Engine.FloatingPawnMovement|SetDeceleration _floatingpawnmovement 2e+02))
  (:Released
    (Variables|/Script/Engine.FloatingPawnMovement|SetMaxSpeed _floatingpawnmovement_2 6e+02)
    (Variables|/Script/Engine.FloatingPawnMovement|SetDeceleration _floatingpawnmovement_2 6e+02)))

(event Input|AxisEvents|InputAxisPitch
  (params (AxisValue :type Float%20%28single-precision%29))
  ;[0.15 0.15 0.15 0.5] 비행기 회전
  (Transformation|AddActorLocalRotation (Math|Rotator|MakeRotator 0.0 (* AxisValue (Utilities|Time|GetWorldDeltaSeconds) (Variables|Default|GetRotationSpeed)) 0.0) false false))

(event Input|AxisEvents|InputAxisRoll
  (params (AxisValue :type Float%20%28single-precision%29))
  ;[0.15 0.15 0.15 0.5] 비행기 회전
  (Transformation|AddActorLocalRotation (Math|Rotator|MakeRotator (* AxisValue (Utilities|Time|GetWorldDeltaSeconds) (Variables|Default|GetRotationSpeed)) 0.0 0.0) false false))

(fn ConstructionScript)

(fn BoostTime
  (bind _floatingpawnmovement (Variables|Default|GetFloatingPawnMovement))
  (Variables|/Script/Engine.FloatingPawnMovement|SetMaxSpeed _floatingpawnmovement 2.4e+03)
  (Variables|/Script/Engine.FloatingPawnMovement|SetAcceleration _floatingpawnmovement 2e+02))